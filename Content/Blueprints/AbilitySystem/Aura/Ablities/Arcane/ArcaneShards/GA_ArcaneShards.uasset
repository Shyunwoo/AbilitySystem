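; Arcane Shards gameplay ability that shows a magic circle, waits for an input press, then erupts a series of shards around the targeted ground point.
; A spawned BP_PointCollection supplies randomly rotated ground points, their count set by ability level up to a cap.
; After the cast montage event, a looping timer spawns each shard as a gameplay cue, dealing radial damage with outward knockback to nearby live players.
; Cooldown commits after the last shard.
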(event Custom|SpawnShard
  (if (< (Variables|Default|GetCount) (Variables|Default|GetNumShards))
    (CallFunction|StoreShardSpawnLocation)
    (CallFunction|StorePlayerstoDamae)
    (for _array_element (Variables|Default|GetPlayersToDamage)
      (CallFunction|RadialDamagetoPlayer _array_element))
    (Math|Integer|IncrementInt (Variables|Default|GetCount)
      (:%20%20
        (Class|GameplayAbility|ExecuteGameplayCuewithParams "(TagName=\"GameplayCue.ArcaneShards\")" (Ability|GameplayCue|MakeGameplayCueParameters :Location (Variables|Default|GetShardSpawnLocation)))))
    (else
      (Utilities|Time|ClearandInvalidateTimerbyHandle (Variables|Default|GetShardSpawnTimer))
      (Actor|DestroyActor (Variables|Default|GetPointCollection))
      (Ability|CommitAbilityCooldown false)
      (Ability|EndAbility))))

(event Ability|EventActivateAbility
  (bind _returnvalue (Class|GameplayAbility|CheckAbilityCost))
  (if _returnvalue
    (Utilities|FlowControl|Sequence
      (:then_0
        (Class|PlayerInterface|ShowMagicCircle(Message) (Ability|GetAvatarActorfromActorInfo) 0))
      (:then_1
        (Ability|Tasks|WaitInputPress false
          (:OnPress
            (bind _datahandle (|TargetDataUnderMouse)
              (:ValidData
                (Variables|Default|SetMouseHitLocation (.ImpactPoint (Collision|BreakHitResult (Ability|TargetData|GetHitResultfromTargetData _datahandle))))
                (Utilities|FlowControl|Sequence
                  (:then_0
                    (bind _returnvalue_2 (Game|SpawnActorfromClass "/Game/Blueprints/AbilitySystem/Aura/Ablities/Arcane/ArcaneShards/BP_PointCollection.BP_PointCollection_C" (Math|Transform|MakeTransform (Variables|Default|GetMouseHitLocation) "0, 0, 0" "1.000000,1.000000,1.000000") "AlwaysSpawn" "MultiplyWithRoot" 0 0))
                    (Variables|Default|SetPointCollection _returnvalue_2)
                    (Variables|Default|SetNumShards (Math|Integer|Min(Integer) (Variables|Default|GetMaxNumShards) (Ability|GetAbilityLevel)))
                    (Variables|Default|SetGroundPoints (Class|PointCollection|GetGroundPoints (Variables|Default|GetPointCollection) (Variables|Default|GetMouseHitLocation) (Variables|Default|GetNumShards) (Math|Random|RandomFloatinRange 0.0 3.6e+02))))
                  (:then_1
                    (Class|CombatInterface|UpdateFacingTarget(Message) (Ability|GetAvatarActorfromActorInfo) (Variables|Default|GetMouseHitLocation)))
                  (:then_2
                    (|PlayMontageandWaitProxy "None" "/Game/Assets/Characters/Aura/Animations/Abilities/AM_Cast_ArcaneShards.AM_Cast_ArcaneShards" 1.0 "None" false 1.0 0.0 false
                      (:then
                        (Ability|Tasks|WaitGameplayEvent "(TagName=\"Event.Montage.ArcaneShards\")" 0 true
                          (:EventReceived
                            (bind _returnvalue_3 (Utilities|Time|SetTimerbyEvent (delegate Custom|SpawnShard) (Variables|Default|GetShardSpawnDeltaTime) true))
                            (Variables|Default|SetShardSpawnTimer _returnvalue_3)
                            (Class|PlayerInterface|HideMagicCircle(Message) (Ability|GetAvatarActorfromActorInfo))
                            (CallFunction|SpawnShard)
                            (Ability|CommitAbilityCost false)))))))))))))))

(fn StoreShardSpawnLocation
  (Variables|Default|SetShardSpawnLocation (Transformation|GetWorldLocation (Utilities|Array|Get(acopy) (Variables|Default|GetGroundPoints) (Variables|Default|GetCount)))))

(fn StorePlayerstoDamae
  (bind _returnvalue (Ability|GetAvatarActorfromActorInfo))
  (bind _outoverlappingactors (Class|AuraAbilitySystemLibrary|GetLivePlayersWithinRadius _returnvalue (Utilities|Array|MakeArray _returnvalue) (Variables|Default|GetRadialDamageOuterRadius) (Variables|Default|GetShardSpawnLocation)))
  (Variables|Default|SetPlayersToDamage _outoverlappingactors))

(fn RadialDamagetoPlayer
  (params (TargetActor :type Actor%20Object%20Reference))
  (bind _returnvalue (Transformation|GetActorLocation TargetActor))
  (bind _shardspawnlocation (Variables|Default|GetShardSpawnLocation))
  (bind _returnvalue_2 (- _returnvalue _shardspawnlocation))
  (Class|AuraAbilitySystemLibrary|ApplyDamageEffect (Class|AuraDamageGameplayAbility|MakeDamageEffectParamsfromClassDefaults TargetActor (Variables|Default|GetShardSpawnLocation) false _returnvalue_2 true _returnvalue_2 true 35.0)))